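; Game state Blueprint for a networked Red-versus-Blue team game that handles the victory outcome and result screen.
; OnVictory walks PlayerArray and notifies each player's avatar, always treating Red as winners and Blue as losers.
; It then creates a result widget for the first local controller, showing a loss message for Blue or the winning player's nickname otherwise.
; OnRestart removes that widget.
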(event EventOnVictory
  (for _array_element (Variables|Default|GetPlayerArray)
    (bind _asnet_player_state (Utilities|Casting|CastToNetPlayerState _array_element))
    (switch Utilities|FlowControl|Switch|SwitchonEPlayerTeam (.teamid (Variables|/Script/Labwork4.NetPlayerState|GetData _asnet_player_state))
      (:TEAM_Blue
        (Default|OnPlayerLost (.AsBP%20Net%20Avatar (Utilities|Casting|CastToBP_NetAvatar (Variables|/Script/Engine.PlayerState|GetPawnPrivate _asnet_player_state)))))
      (:TEAM_Red
        (Default|OnPlayerWon (.AsBP%20Net%20Avatar (Utilities|Casting|CastToBP_NetAvatar (Variables|/Script/Engine.PlayerState|GetPawnPrivate _asnet_player_state)))))))
  (CallFunction|ShowResultScreen))

(event EventOnRestart
  (Widget|RemovefromParent (Variables|Default|GetMessageWidget)))

(fn ConstructionScript)

(fn ShowResultScreen
  (bind _returnvalue (Class|NetGameState|GetPlayerStatebyIndex (Variables|Default|GetWinningPlayer)))
  (bind _returnvalue_2 (UserInterface|CreateWidget "/Game/Blueprints/UMG/W_GameResults.W_GameResults_C" 0 (Utilities|Text|ToText(String) (select (Utilities|Enum|Equal(Enum) (.teamid (Variables|/Script/Labwork4.NetPlayerState|GetData (.AsNet%20Player%20State (Utilities|Casting|CastToNetPlayerState (Variables|/Script/Engine.Controller|GetPlayerState (Game|GetPlayerController 0)))))) "TEAM_Blue") "YouLose!" (Utilities|String|Append (Utilities|String|ToString(Text) (.Nickname (Utilities|Struct|BreakSPlayerInfo (Variables|/Script/Labwork4.NetPlayerState|GetData _returnvalue)))) "Wins")))))
  (Variables|Default|SetMessageWidget _returnvalue_2)
  (UserInterface|Viewport|AddtoViewport _returnvalue_2 0))