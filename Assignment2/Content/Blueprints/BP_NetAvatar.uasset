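; Networked team-game player avatar that reports avatar overlaps to the game mode and gives Red-team players a forward dash.
; Tick line-traces ahead for a tag-checked hit, setting a destination short of it by the capsule radius.
; Dash input passes through server and client events to a timeline that lerps location in Flying mode, with montage and timeline rates scaled by distance.
; Player-state changes recolor body materials by team; win/loss events stop dashing or disable input.
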(event Custom|AllowDash
  ;[1 1 1] Comment
  (Variables|Default|SetMovementScale 1.0)
  (Actor|Tick|SetActorTickEnabled true)
  (Utilities|FlowControl|DoOnce false) ; enters at Reset
)

(event Custom|DoDashServer
  ;[1 1 1] Comment
  (CallFunction|DoDashClient (Variables|Default|GetDashSource) (Variables|Default|GetDashDestination)))

(event Custom|DoDashClient
  (params (Source :type Vector) (Destination :type Vector))
  (bind _dashdistance (Variables|Default|GetDashDistance))
  (bind _returnvalue (/ 1e+03 _dashdistance))
  ;[1 1 1] Comment
  (Variables|Default|SetDashSource Source)
  (Variables|Default|SetDashDestination Destination)
  (Animation|PlayAnimMontage "/Game/Mannequin/Animations/AM_Dash.AM_Dash" (* _returnvalue 1.4) "None")
  (Pawn|Components|CharacterMovement|SetMovementMode (Variables|Character|GetCharacterMovement) "MOVE_Flying" 0)
  (Variables|Default|SetDashSource (Transformation|GetActorLocation))
  (Variables|Default|SetMovementScale 0.0)
  (Actor|Tick|SetActorTickEnabled false)
  (Components|Timeline|SetPlayRate (Variables|Default|GetDashAnim) _returnvalue)
  (bind _newtrack_0 (Timeline|DashAnim Play)
    (:Update
      (Transformation|SetActorLocation (Math|Vector|Lerp(Vector) (Variables|Default|GetDashSource) (Variables|Default|GetDashDestination) _newtrack_0) false true))
    (:Finished
      (Pawn|Components|CharacterMovement|SetMovementMode (Variables|Character|GetCharacterMovement) "MOVE_Walking" 0)
      (CallFunction|AllowDash))))

(event Custom|Victory
  ;[1 1 1] Comment
  (bind _newtrack_0 (Timeline|DashAnim Stop)
    (:Update
      (Transformation|SetActorLocation (Math|Vector|Lerp(Vector) (Variables|Default|GetDashSource) (Variables|Default|GetDashDestination) _newtrack_0) false true))
    (:Finished
      (Pawn|Components|CharacterMovement|SetMovementMode (Variables|Character|GetCharacterMovement) "MOVE_Walking" 0)
      (CallFunction|AllowDash))))

(event Custom|Defeat
  ;[1 1 1] Comment
  (Input|DisableInput (Game|GetPlayerController 0))
  (Physics|SetSimulatePhysics (Variables|Character|GetMesh) false)
  (Collision|SetCollisionResponsetoChannel (Variables|Default|GetCapsuleComponent) "ECC_PhysicsBody" "ECR_Ignore"))

(event Custom|OnPlayerWon
  ;[1 1 1] Comment
  (CallFunction|Victory))

(event Custom|OnPlayerLost
  ;[1 1 1] Comment
  (CallFunction|Defeat))

(event EventBeginPlay)

(event Collision|EventActorBeginOverlap
  (params (OtherActor :type Actor%20Object%20Reference))
  ;[1 1 1] Comment
  (bind _asbp_net_game_mode (Utilities|Casting|CastToBP_NetGameMode (Game|GetGameMode)))
  (bind _asnet_avatar (Utilities|Casting|CastToNetAvatar OtherActor))
  (Class|NetGameMode|AvatarsOverlapped _asbp_net_game_mode self _asnet_avatar))

(event EventTick
  (params (DeltaSeconds :type Float%20%28single-precision%29))
  (bind _returnvalue (Transformation|GetActorLocation))
  ;[1 1 1] Comment
  (Variables|Default|SetDashOK false)
  (bind _asnet_player_state (Utilities|PState)
    (:%20%20
      (switch Utilities|FlowControl|Switch|SwitchonEPlayerTeam (.teamid (Variables|/Script/Labwork4.NetPlayerState|GetData _asnet_player_state))
        (:TEAM_Red
          (bind (_outhit _returnvalue_2) (Collision|LineTraceByChannel _returnvalue (+ _returnvalue (* (Transformation|GetActorForwardVector) 3e+03)) "TraceTypeQuery1" false 0 "ForDuration"))
          (if _returnvalue_2
            (if (Actor|ActorHasTag (.HitActor (Collision|BreakHitResult _outhit)) "None")
              (Variables|Default|SetDashDistance (.Distance (Collision|BreakHitResult _outhit)))
              (Variables|Default|SetDashDestination (Math|Vector|MakeVector (.X (Math|Vector|BreakVector (- (.Location (Collision|BreakHitResult _outhit)) (* (Transformation|GetActorForwardVector) (Variables|/Script/Engine.CapsuleComponent|GetCapsuleRadius (Variables|Default|GetCapsuleComponent)))))) (.Y (Math|Vector|BreakVector (- (.Location (Collision|BreakHitResult _outhit)) (* (Transformation|GetActorForwardVector) (Variables|/Script/Engine.CapsuleComponent|GetCapsuleRadius (Variables|Default|GetCapsuleComponent)))))) (.z (Transformation|GetActorLocation))))
              (Variables|Default|SetDashOK true))))))))

(event EventOnPlayerInfoChanged
  (bind _mesh (Variables|Character|GetMesh))
  ;[1 1 1] Comment
  (bind _asnet_player_state (Utilities|PState)
    (:%20%20
      (Rendering|Material|SetVectorParameterValueonMaterials _mesh "Color 1" (Utilities|Select :Index (.teamid (Variables|/Script/Labwork4.NetPlayerState|GetData _asnet_player_state)) :TEAM_Unknown "0, 0, 0" :TEAM_Blue "0, 0, 0" :TEAM_Red "0, 0, 0"))
      (Rendering|Material|SetVectorParameterValueonMaterials _mesh "Color 2" (Utilities|Select :Index (.teamid (Variables|/Script/Labwork4.NetPlayerState|GetData _asnet_player_state)) :TEAM_Unknown "0, 0, 0" :TEAM_Blue "0, 0, 0" :TEAM_Red "0, 0, 0"))
      (Rendering|Material|SetVectorParameterValueonMaterials _mesh "Color 3" (Utilities|Select :Index (.teamid (Variables|/Script/Labwork4.NetPlayerState|GetData _asnet_player_state)) :TEAM_Unknown "0, 0, 0" :TEAM_Blue "0, 0, 0" :TEAM_Red "0, 0, 0")))))

(event Input|ActionEvents|InputActionDash
  (params (Key :type Key%20Structure :default "None"))
  ;[1 1 1] Comment
  (:Pressed
    (if (Variables|Default|GetDashOK)
      (Utilities|FlowControl|DoOnce false
        (:Completed
          (CallFunction|DoDashServer))))))

(fn ConstructionScript)